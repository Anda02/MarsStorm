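; Actor Blueprint for an Oberth ship cloak effect, toggled with the C key.
; BeginPlay enables player input and creates a dynamic instance of the Shipcloak material.
; A FlipFlop plays or reverses the Fade timeline, whose value drives a scalar material parameter on Dmi.
; The nodes that store the instance in Dmi and apply it to the mesh are disconnected, so they never run.
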(event EventBeginPlay
  (Input|EnableInput (Game|GetPlayerController 0))
  (bind _returnvalue (Rendering|Material|CreateDynamicMaterialInstance "/Game/Materials/shipcloak.shipcloak" :!class /Script/Engine.KismetMaterialLibrary)))

(event Collision|EventActorBeginOverlap
  (params (OtherActor :type Actor%20Object%20Reference)))

(event EventTick
  (params (DeltaSeconds :type Float%20%28single-precision%29)))

(event Input|KeyboardEvents|C
  (params (Key :type Key%20Structure :default "AnyKey"))
  (:Pressed
    (Utilities|FlowControl|FlipFlop
      (:A
        (bind _fadetime (Timeline|Fade Play)
          (:Update
            (Rendering|Material|SetScalarParameterValue (Variables|Default|Getdmi) "None_1" _fadetime :!class /Script/Engine.MaterialInstanceDynamic))))
      (:B
        (Timeline|Fade Reverse)))))

(fn ConstructionScript)